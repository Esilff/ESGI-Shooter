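; BP_MasterBonus is a respawning pickup that grants the player ammunition or health, selected by EBonusType.
; Sphere overlap with BP_Player applies the bonus, plays a short spark burst and sound, then hides the actor and disables its collision.
; After CoolDownBonus, it reappears with collision and another spark burst.
; A sine-based movement offset is left unconnected, so Tick does nothing.
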(event OnComponentBeginOverlap(Sphere)
  (params (OverlappedComponent :type Primitive%20Component%20Object%20Reference) (OtherActor :type Actor%20Object%20Reference) (OtherComp :type Primitive%20Component%20Object%20Reference) (OtherBodyIndex :type Integer) (bFromSweep :type Boolean) (SweepResult :type Hit%20Result%20Structure%20%28by%20ref%29))
  (bind _asbp_player (Utilities|Casting|CastToBP_Player OtherActor))
  (switch Utilities|FlowControl|Switch|SwitchonE_BonusType (Variables|Default|GetE_BonusType)
    (:NewEnumerator0
      (Default|AddBullets _asbp_player (Variables|Default|GetBulletsToAdd)))
    (:NewEnumerator1
      (Default|AddHealth _asbp_player (Variables|Default|GetHealthToAdd))))
  (bind _returnvalue (Effects|SpawnEmitteratLocation "/Game/StarterContent/Particles/P_Sparks.P_Sparks" (Transformation|GetActorLocation) "0, 0, 0" "5.000000,5.000000,5.000000"))
  (Utilities|FlowControl|Sequence
    (:then_0
      (Utilities|FlowControl|Delay 0.2)
      (Components|DestroyComponent _returnvalue))
    (:then_1
      (Audio|PlaySoundatLocation "/Game/StarterContent/Audio/Collapse01.Collapse01" (Transformation|GetActorLocation) "0, 0, 0" 0.1 1.0 0.0 0 0 0 0))
    (:then_2
      (Rendering|SetActorHiddenInGame true)
      (Collision|SetActorEnableCollision false))
    (:then_3
      (Utilities|FlowControl|Delay (Variables|Default|GetCoolDownBonus))
      (Rendering|SetActorHiddenInGame false)
      (Collision|SetActorEnableCollision true)
      (bind _returnvalue_2 (Effects|SpawnEmitteratLocation "/Game/StarterContent/Particles/P_Sparks.P_Sparks" (Transformation|GetActorLocation) "0, 0, 0" "5.000000,5.000000,5.000000"))
      (Utilities|FlowControl|Delay 0.2)
      (Components|DestroyComponent _returnvalue_2))))

(event EventTick
  (params (DeltaSeconds :type Float%20%28single-precision%29)))

(fn ConstructionScript)
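; Gamemode Blueprint that tracks game time and the charge meter for a toggleable Sandevistan ability.
; Until game over, Tick advances the timer and updates the meter, draining it while active and refilling it toward the cooldown limit otherwise.
; The Sandevistan event only flips the active state, with no further effect here, and fires automatically when the meter empties.
; CooldownRatio exposes the normalized charge.
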(event Custom|Sandevistan
  (bind _output_get (Variables|Default|SetsandevistanActive (not (Variables|Default|GetsandevistanActive))))
  (if _output_get
    _))

(event EventTick
  (params (DeltaSeconds :type Float%20%28single-precision%29))
  (if (not (Variables|Default|GetgameOver))
    (Variables|Default|Settimer (+ (Variables|Default|Gettimer) DeltaSeconds))
    (CallFunction|CheckSandevistan DeltaSeconds DeltaSeconds)))

(fn ConstructionScript)

(fn CooldownRatio
  (return (/ (Variables|Default|GetCurrentCooldown) (Variables|Default|GetCooldown))))

(fn CheckSandevistan
  (params (A :type Float%20%28double-precision%29) (B :type Float%20%28double-precision%29))
  (if (Variables|Default|GetsandevistanActive)
    (Variables|Default|SetCurrentCooldown (- (Variables|Default|GetCurrentCooldown) (* A 1.0)))
    (if (<= (Variables|Default|GetCurrentCooldown) 0.0)
      (CallFunction|Sandevistan))
    (elif (< (Variables|Default|GetCurrentCooldown) (Variables|Default|GetCooldown))
      (Variables|Default|SetCurrentCooldown (+ (Variables|Default|GetCurrentCooldown) B)))))
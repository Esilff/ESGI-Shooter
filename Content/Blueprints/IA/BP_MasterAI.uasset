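; Master enemy AI character whose IAType enum (short, middle or long range) sets health, gun range, reload and bullet damage.
; AI Perception drives a recursive event loop: chase the player into range and fire BP_Bullet, seek around the last seen location with a doubling radius, or patrol randomly.
; Bullet overlaps reduce health until it explodes and is destroyed.
; Tick lowers CustomTimeDilation while the GameMode's Sandevistan slow-motion is active.
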(event OnTargetPerceptionInfoUpdated(AIPerception)
  (params (UpdateInfo :type Actor%20Perception%20Update%20Info%20Structure%20%28by%20ref%29))
  ;[1 1 1] If we see player and we are not in range get closer to fire - if we don't see player seek for him or patrol
  (if (and (== (.target UpdateInfo) (Game|GetPlayerCharacter 0)) (.bsuccessfullysensed (.stimulus UpdateInfo)))
    (Variables|Perception|SetcanSeePlayer? true)
    (Utilities|AmIinGunRange?
      (:ImNotInRange
        (CallFunction|GotoPlayerLocationNotinGunRange (.stimuluslocation (.stimulus UpdateInfo))))
      (:AmInRange
        (CallFunction|Fire)))
    (else
      (Variables|Perception|SetcanSeePlayer? false)
      (if (<= (Variables|NbSeekPlayerIteration|Getnb_seekPlayer) (Variables|nbSeekPlayerIteration|Getnb_seekPlayerIterationMax))
        (CallFunction|SeekPlayer (.stimuluslocation (.stimulus UpdateInfo)))
        (else
          (CallFunction|ReturntoPatrol))))))

(event OnComponentBeginOverlap(CapsuleComponent)
  (params (OverlappedComponent :type Primitive%20Component%20Object%20Reference) (OtherActor :type Actor%20Object%20Reference) (OtherComp :type Primitive%20Component%20Object%20Reference) (OtherBodyIndex :type Integer) (bFromSweep :type Boolean) (SweepResult :type Hit%20Result%20Structure%20%28by%20ref%29))
  (bind _returnvalue (Transformation|GetActorLocation))
  ;[1 1 1] Check if we overlap a bp bullet - decrease life - if we are dead, play sfx/vfx + destroy actor
  (bind _asbp_bullet (Utilities|Casting|CastToBP_Bullet OtherActor))
  (bind _output_get (Variables|CharacterInfo|Sethealth (- (Variables|CharacterInfo|Gethealth) (Variables|/Game/Blueprints/Weapons/BP_Bullet.BP_Bullet_C|Getdamage _asbp_bullet))))
  (if (<= _output_get 0.0)
    (Effects|SpawnEmitteratLocation "/Game/StarterContent/Particles/P_Explosion.P_Explosion" _returnvalue)
    (Audio|PlaySoundatLocation "/Game/StarterContent/Audio/Explosion01.Explosion01" _returnvalue "0, 0, 0" 1.0 1.0 0.0 0 0 0 0)
    (Default|CallDeath)
    (Actor|DestroyActor _asbp_bullet)
    (Actor|DestroyActor)
    (else
      (Development|PrintString (Utilities|String|Append "IA hp left: " (Utilities|String|ToString(Float) (Variables|CharacterInfo|Gethealth)))))))

(event Custom|SeekPlayer
  (params (LastSeenPlayerLocation :type Vector))
  ;[1 1 1] Increase radius random point - increase iteration check - return patrol or seek player
  (Utilities|FlowControl|Delay (Math|Random|RandomFloatinRange 2.0 5.0))
  (Development|PrintString "SeekPlayer")
  (Variables|RadiusRandomReachablePoint|SetRadiusLookingForPlayer (* (Variables|RadiusRandomReachablePoint|GetRadiusLookingForPlayer) 2.0))
  (bind _result (Math|Integer|IncrementInt (Variables|NbSeekPlayerIteration|Getnb_seekPlayer))
    (:%20%20
      (if (>= _result (Variables|nbSeekPlayerIteration|Getnb_seekPlayerIterationMax))
        (CallFunction|ReturntoPatrol)
        (else
          (CallFunction|SeekPlayerMoveto LastSeenPlayerLocation))))))

(event Custom|SeekPlayerMoveTo
  (params (LastSeenPlayerLocation :type Vector))
  (bind _radiuslookingforplayer (Variables|RadiusRandomReachablePoint|GetRadiusLookingForPlayer))
  (bind _randomlocation (AI|Navigation|GetRandomReachablePointinRadius LastSeenPlayerLocation _radiuslookingforplayer 0 0))
  ;[1 1 1] Get a random point in a radius from last seen player location - move ia to the random point
  (Development|PrintString "SeekPlayerMoveTo")
  (AI|AIMoveTo self _randomlocation 0 5.0 false
    (:OnSuccess
      _)
    (:OnFail
      _))
  (CallFunction|CheckCanSeePlayerFireGunRange _randomlocation))

(event Custom|ReturnToPatrol
  ;[1 1 1] Patrol - Get random point in area
  (Development|PrintString "Return to patrol")
  (Variables|NbSeekPlayerIteration|Setnb_seekPlayer 0)
  (AI|AIMoveTo self (.RandomLocation (AI|Navigation|GetRandomReachablePointinRadius (Transformation|GetActorLocation) (Variables|RadiusRandomReachablePoint|GetRadiusPatrol) 0 0)) 0 5.0 false
    (:OnSuccess
      _)
    (:OnFail
      _))
  (Utilities|FlowControl|Delay (Math|Random|RandomFloatinRange 2.0 5.0))
  (CallFunction|ReturntoPatrol))

(event Custom|GoToPlayerLocation_NotInGunRange
  (params (LastPlayerLocation :type Vector))
  ;[1 1 1] move ia to last seen player location
  (AI|AIMoveTo self LastPlayerLocation 0 (Variables|FireRange|GetGunRange) false
    (:then
      (Variables|Perception|SetMoving? true))
    (:OnSuccess
      (Variables|Perception|SetMoving? false :!label _label)
      (CallFunction|CheckCanSeePlayerFireGunRange LastPlayerLocation))
    (:OnFail
      (goto _label))))

(event Custom|Fire
  ;[1 1 1] Fire bullet - stop movement - rotate to player - spawn bp bullet
  (Development|PrintString "GunFire")
  (Components|Movement|StopMovementImmediately (Variables|Character|GetCharacterMovement))
  (Transformation|SetActorRotation (Math|Rotator|MakeRotator 0.0 0.0 (.yaw (Math|Rotator|FindLookatRotation (Transformation|GetActorLocation) (Transformation|GetActorLocation (Game|GetPlayerCharacter 0))))))
  (Game|SpawnActorfromClass "/Game/Blueprints/Weapons/BP_Bullet.BP_Bullet_C" (Transformation|GetWorldTransform (Variables|Default|GetBulletSpawner)) "Undefined" "MultiplyWithRoot" 0 (Variables|GunFire|GetBulletDamage) true 0)
  (Utilities|FlowControl|Delay (Variables|GunFire|GetReloadDelay))
  (CallFunction|CheckCanSeePlayerFireGunRange (Transformation|GetActorLocation)))

(event EventBeginPlay
  ;[1 1 1] Set variables from our enum ai type
  (switch Utilities|FlowControl|Switch|SwitchonE_IA_Type (Variables|CharacterInfo|GetIA_Type)
    (:NewEnumerator0
      (Variables|FireRange|SetGunRange (Variables|FireRange|GetGunRange_Middle))
      (Variables|GunFire|SetReloadDelay 0.3)
      (bind _output_get (Variables|characterinfo|SethealthMax 1.5e+02))
      (Variables|CharacterInfo|Sethealth _output_get)
      (Variables|GunFire|SetBulletDamage 1e+01))
    (:NewEnumerator1
      (Variables|FireRange|SetGunRange (Variables|FireRange|GetGunRange_Long))
      (Variables|GunFire|SetReloadDelay 4.0)
      (bind _output_get_2 (Variables|characterinfo|SethealthMax 5e+01))
      (Variables|CharacterInfo|Sethealth _output_get_2)
      (Variables|GunFire|SetBulletDamage 1e+02))
    (:NewEnumerator2
      (Variables|FireRange|SetGunRange (Variables|Firerange|GetGunRange_Short))
      (Variables|GunFire|SetReloadDelay 2.5)
      (bind _output_get_3 (Variables|characterinfo|SethealthMax 3e+02))
      (Variables|CharacterInfo|Sethealth _output_get_3)
      (Variables|GunFire|SetBulletDamage 2e+01))))

(event EventTick
  (params (DeltaSeconds :type Float%20%28single-precision%29))
  (bind _assandevistan (Utilities|Casting|CastToSandevistan (Game|GetGameMode)))
  (if (Variables|/Game/Blueprints/Gamemode/Sandevistan.Sandevistan_C|GetsandevistanActive _assandevistan)
    (Variables|Default|SetCustomTimeDilation 0.1)
    (else
      (Variables|Default|SetCustomTimeDilation 1.0))))

(fn ConstructionScript)

(fn RotatetoPlayer
  (if (Variables|Perception|GetcanSeePlayer?)
    (Transformation|SetActorRotation (Math|Rotator|FindLookatRotation (Transformation|GetActorLocation) (Transformation|GetActorLocation (Game|GetPlayerCharacter 0))))
    (else
      (Utilities|Time|ClearTimerbyFunctionName 0 "RotateToPlayer"))))

(fn CheckCanSeePlayerFireGunRange
  (params (LastSeenPlayerLocation :type Vector))
  (if (Variables|Perception|GetcanSeePlayer?)
    (Utilities|AmIinGunRange?
      (:ImNotInRange
        (CallFunction|SeekPlayer LastSeenPlayerLocation :!label _label))
      (:AmInRange
        (CallFunction|Fire)))
    (else
      (goto _label))))
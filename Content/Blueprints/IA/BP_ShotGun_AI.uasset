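; AI shotgun weapon Blueprint that fires four bullets per shot.
; Its Fire event calls the parent implementation, then spawns a BP_Bullet at each of four BulletSpawner transforms, passing BulletDamage to every bullet.
; Only the bullet from the first spawner is spawned with SandevistanSlowed set to true.
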(event EventBeginPlay
  (|CallParentFunction) ; This node is disabled and will not be called.\nDrag off pins to build functionality.
)

(event Collision|EventActorBeginOverlap
  (params (OtherActor :type Actor%20Object%20Reference)))

(event EventTick
  (params (DeltaSeconds :type Float%20%28single-precision%29)))

(event EventFire
  (|CallParentFunction)
  (Game|SpawnActorfromClass "/Game/Blueprints/Weapons/BP_Bullet.BP_Bullet_C" (Transformation|GetWorldTransform (Variables|Default|GetBulletSpawner1)) "Undefined" "MultiplyWithRoot" 0 (Variables|Default|GetBulletDamage) true 0)
  (Game|SpawnActorfromClass "/Game/Blueprints/Weapons/BP_Bullet.BP_Bullet_C" (Transformation|GetWorldTransform (Variables|Default|GetBulletSpawner2)) "Undefined" "MultiplyWithRoot" 0 (Variables|Default|GetBulletDamage) false 0)
  (Game|SpawnActorfromClass "/Game/Blueprints/Weapons/BP_Bullet.BP_Bullet_C" (Transformation|GetWorldTransform (Variables|Default|GetBulletSpawner3)) "Undefined" "MultiplyWithRoot" 0 (Variables|Default|GetBulletDamage) false 0)
  (Game|SpawnActorfromClass "/Game/Blueprints/Weapons/BP_Bullet.BP_Bullet_C" (Transformation|GetWorldTransform (Variables|Default|GetBulletSpawner4)) "Undefined" "MultiplyWithRoot" 0 (Variables|Default|GetBulletDamage) false 0))

(fn ConstructionScript
  (|CallParentFunction))